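; Snappy Roads vehicle actor that drives at constant speed along the splines of the roads in FollowPath, forward or in reverse, looping at the ends.
; BeginPlay sets the start road and distance from StartAtRoad and TimeOffset, and shifts the decal to fit mesh bounds.
; Tick places it by spline distance with lane offset, or destroys it if the path is empty.
; Gaps between roads are bridged by tangent-matched splines, built at runtime and cached in TempSpline.
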(event EventBeginPlay
  (Utilities|FlowControl|Delay 0.0)
  (Utilities|FlowControl|Sequence
    (:then_0
      (Transformation|AddRelativeLocation (Variables|Default|GetDecal) (Math|Vector|MakeVector (- (Math|Float|Absolute(Float) (.x (.Min (Components|StaticMesh|GetLocalBounds (Variables|Default|GetStaticMesh))))) 2.1e+02) 0.0 0.0) false false))
    (:then_1
      (Development|PrintString (Utilities|String|ToString(Float) (Variables|Default|GetTimeOffset)))
      (Utilities|FlowControl|Sequence
        (:then_0
          (Variables|Default|SetCurrentRoad (Math|Integer|%(Integer) (Variables|Default|GetStartAtRoad) (Utilities|Array|Length (Variables|Default|GetFollowPath)))))
        (:then_1
          ;[1 1 1] RandomOffset
          (Variables|Default|SetCurrentDistance (Math|Float|%(Float) (* (Variables|Default|GetTimeOffset) (/ (* (Variables|Default|GetSpeed%28km/h%29) 1e+03 1e+02) 3.6e+03)) (Spline|GetSplineLength (Variables|/Game/SnappyRoads/Blueprints/BP_SnappyRoad.BP_SnappyRoad_C|GetSpline (Utilities|Array|Get(acopy) (Variables|Default|GetFollowPath) (Variables|Default|GetCurrentRoad)))))))))))

(event Collision|EventActorBeginOverlap
  (params (OtherActor :type Actor%20Object%20Reference)))

(event EventTick
  (params (DeltaSeconds :type Float%20%28single-precision%29))
  (bind _followpath (Variables|Default|GetFollowPath))
  (bind _speed_km_h_ (Variables|Default|GetSpeed%28km/h%29))
  (bind _followpath_2 (Variables|Default|GetFollowPath))
  (bind _followpath_3 (Variables|Default|GetFollowPath))
  (bind _returnvalue (Utilities|Array|Length _followpath_3))
  (bind _returnvalue_2 (Utilities|Array|Length _followpath))
  (bind _returnvalue_3 (* _speed_km_h_ 1e+03 1e+02))
  (bind _returnvalue_4 (/ _returnvalue_3 3.6e+03))
  (bind _returnvalue_5 (* DeltaSeconds _returnvalue_4))
  ;[1 1 1] Destroy If Old
  (if (> (Utilities|Array|Length _followpath_2) 0)
    (if (Variables|Default|GetReverse)
      ;[1 1 1] Reverse
      ;;[1 1 1] AdvanceR
      (Variables|Default|SetCurrentDistance (- (Variables|Default|GetCurrentDistance) _returnvalue_5))
      ;;[1 1 1] EndReached?
      (if (<= (Variables|Default|GetCurrentDistance) 0.0)
        ;;[1 1 1] EndOfJoiningSpline
        (if (Variables|Default|GetStateReaching)
          (Variables|Default|SetStateReaching false)
          (bind _output_get (Variables|Default|SetCurrentRoad (Math|Integer|Absolute(Integer) (Math|Integer|%(Integer) (- (Variables|Default|GetCurrentRoad) 1) _returnvalue))))
          (Variables|Default|SetCurrentDistance (Spline|GetSplineLength (Variables|/Game/SnappyRoads/Blueprints/BP_SnappyRoad.BP_SnappyRoad_C|GetSpline (Utilities|Array|Get(acopy) _followpath_3 _output_get))))
          (else
            ;;[1 1 1] EndOfLastSpline
            (if (<= (Variables|Default|GetCurrentRoad) 0)
              (bind _output_get_2 (Variables|Default|SetCurrentRoad (- _returnvalue 1)))
              (Variables|Default|SetCurrentDistance (Spline|GetSplineLength (Variables|/Game/SnappyRoads/Blueprints/BP_SnappyRoad.BP_SnappyRoad_C|GetSpline (Utilities|Array|Get(acopy) _followpath_3 _output_get_2))))
              (else
                (Variables|Default|SetStateReaching true)
                (Utilities|IsValid (Utilities|Array|Get(acopy) (Variables|Default|GetTempSpline) (Variables|Default|GetCurrentRoad))
                  (:Is%20Valid
                    _)
                  (:Is%20Not%20Valid
                    ;;[1 1 1] ConstructJoiningSpline
                    (bind _returnvalue_6 (AddComponent|AddSplineComponent (Utilities|Array|Get(acopy) (Variables|Default|GetFollowPath) (Math|Integer|Absolute(Integer) (Math|Integer|%(Integer) (- (Variables|Default|GetCurrentRoad) 1) _returnvalue))) false (Spline|GetTransformatSplinePoint (Variables|/Game/SnappyRoads/Blueprints/BP_SnappyRoad.BP_SnappyRoad_C|GetSpline (Utilities|Array|Get(acopy) (Variables|Default|GetFollowPath) (Math|Integer|Absolute(Integer) (Math|Integer|%(Integer) (- (Variables|Default|GetCurrentRoad) 1) _returnvalue)))) (- (Spline|GetNumberOfSplinePoints (Variables|/Game/SnappyRoads/Blueprints/BP_SnappyRoad.BP_SnappyRoad_C|GetSpline (Utilities|Array|Get(acopy) (Variables|Default|GetFollowPath) (Math|Integer|Absolute(Integer) (Math|Integer|%(Integer) (- (Variables|Default|GetCurrentRoad) 1) _returnvalue))))) 1) "Local" false)))
                    (Utilities|Array|SetArrayElem (Variables|Default|GetTempSpline) (Variables|Default|GetCurrentRoad) _returnvalue_6 true)
                    (Spline|SetLocationatSplinePoint _returnvalue_6 1 (Spline|GetLocationatSplinePoint (Variables|/Game/SnappyRoads/Blueprints/BP_SnappyRoad.BP_SnappyRoad_C|GetSpline (Utilities|Array|Get(acopy) (Variables|Default|GetFollowPath) (Variables|Default|GetCurrentRoad))) 0 "World") "World" true)
                    (Spline|SetTangentatSplinePoint _returnvalue_6 0 (* (Math|Vector|Normalize (Spline|GetTangentatSplinePoint (Variables|/Game/SnappyRoads/Blueprints/BP_SnappyRoad.BP_SnappyRoad_C|GetSpline (Utilities|Array|Get(acopy) (Variables|Default|GetFollowPath) (Math|Integer|Absolute(Integer) (Math|Integer|%(Integer) (- (Variables|Default|GetCurrentRoad) 1) _returnvalue)))) (- (Spline|GetNumberOfSplinePoints (Variables|/Game/SnappyRoads/Blueprints/BP_SnappyRoad.BP_SnappyRoad_C|GetSpline (Utilities|Array|Get(acopy) (Variables|Default|GetFollowPath) (Math|Integer|Absolute(Integer) (Math|Integer|%(Integer) (- (Variables|Default|GetCurrentRoad) 1) _returnvalue))))) 1) "World")) (Spline|GetSplineLength _returnvalue_6)) "World" false)
                    (Spline|SetTangentatSplinePoint _returnvalue_6 1 (* (Math|Vector|Normalize (Spline|GetTangentatSplinePoint (Variables|/Game/SnappyRoads/Blueprints/BP_SnappyRoad.BP_SnappyRoad_C|GetSpline (Utilities|Array|Get(acopy) (Variables|Default|GetFollowPath) (Variables|Default|GetCurrentRoad))) 0 "World")) (Spline|GetSplineLength _returnvalue_6)) "World" true)))
                (Variables|Default|SetCurrentDistance (Spline|GetSplineLength (Utilities|Array|Get(acopy) (Variables|Default|GetTempSpline) (Variables|Default|GetCurrentRoad))))))))
        (else
          ;[1 1 1] MoveActor
          (Transformation|SetActorLocationAndRotation (+ (Spline|GetLocationatDistanceAlongSpline (select (Variables|Default|GetStateReaching) (Utilities|Array|Get(acopy) (Variables|Default|GetTempSpline) (Variables|Default|GetCurrentRoad)) (Variables|/Game/SnappyRoads/Blueprints/BP_SnappyRoad.BP_SnappyRoad_C|GetSpline (Utilities|Array|Get(acopy) _followpath_2 (Variables|Default|GetCurrentRoad)))) (stale _output_get_3) "World") (Math|Vector|RotateVector (+ (Variables|Default|GetOffset) (Math|Vector|MakeVector 0.0 (* (Variables|Default|GetLane) (Variables|Default|GetLineWidth)) 0.0)) (Math|Conversions|RotationFromXVector (select (Variables|Default|GetReverse) (Math|Vector|NegateVector (Spline|GetTangentatDistanceAlongSpline (select (Variables|Default|GetStateReaching) (Utilities|Array|Get(acopy) (Variables|Default|GetTempSpline) (Variables|Default|GetCurrentRoad)) (Variables|/Game/SnappyRoads/Blueprints/BP_SnappyRoad.BP_SnappyRoad_C|GetSpline (Utilities|Array|Get(acopy) _followpath_2 (Variables|Default|GetCurrentRoad)))) (stale _output_get_3) "World")) (Spline|GetTangentatDistanceAlongSpline (select (Variables|Default|GetStateReaching) (Utilities|Array|Get(acopy) (Variables|Default|GetTempSpline) (Variables|Default|GetCurrentRoad)) (Variables|/Game/SnappyRoads/Blueprints/BP_SnappyRoad.BP_SnappyRoad_C|GetSpline (Utilities|Array|Get(acopy) _followpath_2 (Variables|Default|GetCurrentRoad)))) (stale _output_get_3) "World"))))) (Math|Conversions|RotationFromXVector (select (Variables|Default|GetReverse) (Math|Vector|NegateVector (Spline|GetTangentatDistanceAlongSpline (select (Variables|Default|GetStateReaching) (Utilities|Array|Get(acopy) (Variables|Default|GetTempSpline) (Variables|Default|GetCurrentRoad)) (Variables|/Game/SnappyRoads/Blueprints/BP_SnappyRoad.BP_SnappyRoad_C|GetSpline (Utilities|Array|Get(acopy) _followpath_2 (Variables|Default|GetCurrentRoad)))) (stale _output_get_3) "World")) (Spline|GetTangentatDistanceAlongSpline (select (Variables|Default|GetStateReaching) (Utilities|Array|Get(acopy) (Variables|Default|GetTempSpline) (Variables|Default|GetCurrentRoad)) (Variables|/Game/SnappyRoads/Blueprints/BP_SnappyRoad.BP_SnappyRoad_C|GetSpline (Utilities|Array|Get(acopy) _followpath_2 (Variables|Default|GetCurrentRoad)))) (stale _output_get_3) "World"))) :!label _label)))
      (else
        ;[1 1 1] Advance
        (bind _output_get_3 (Variables|Default|SetCurrentDistance (+ (Variables|Default|GetCurrentDistance) _returnvalue_5)))
        ;[1 1 1] EndReached?
        (if (>= _output_get_3 (Spline|GetSplineLength (select (Variables|Default|GetStateReaching) (Utilities|Array|Get(acopy) (Variables|Default|GetTempSpline) (Variables|Default|GetCurrentRoad)) (Variables|/Game/SnappyRoads/Blueprints/BP_SnappyRoad.BP_SnappyRoad_C|GetSpline (Utilities|Array|Get(acopy) _followpath_2 (Variables|Default|GetCurrentRoad))))))
          (Variables|Default|SetCurrentDistance 0.0)
          ;[1 1 1] EndOfJoiningSpline?
          (if (Variables|Default|GetStateReaching)
            (Variables|Default|SetStateReaching false)
            (Variables|Default|SetCurrentRoad (Math|Integer|%(Integer) (+ (Variables|Default|GetCurrentRoad) 1) _returnvalue_2))
            (else
              ;[1 1 1] EndOfLastSpline?
              (if (>= (Variables|Default|GetCurrentRoad) (- _returnvalue_2 1))
                (Variables|Default|SetCurrentRoad 0)
                (else
                  (Variables|Default|SetStateReaching true)
                  (Utilities|IsValid (Utilities|Array|Get(acopy) (Variables|Default|GetTempSpline) (Variables|Default|GetCurrentRoad))
                    (:Is%20Not%20Valid
                      ;[1 1 1] ConstructJoiningSpline
                      (bind _returnvalue_7 (AddComponent|AddSplineComponent (Utilities|Array|Get(acopy) _followpath (Variables|Default|GetCurrentRoad)) false (Spline|GetTransformatSplinePoint (Variables|/Game/SnappyRoads/Blueprints/BP_SnappyRoad.BP_SnappyRoad_C|GetSpline (Utilities|Array|Get(acopy) _followpath (Variables|Default|GetCurrentRoad))) (- (Spline|GetNumberOfSplinePoints (Variables|/Game/SnappyRoads/Blueprints/BP_SnappyRoad.BP_SnappyRoad_C|GetSpline (Utilities|Array|Get(acopy) _followpath (Variables|Default|GetCurrentRoad)))) 1) "Local" false)))
                      (Utilities|Array|SetArrayElem (Variables|Default|GetTempSpline) (Variables|Default|GetCurrentRoad) _returnvalue_7 true)
                      (Spline|SetLocationatSplinePoint _returnvalue_7 1 (Spline|GetLocationatSplinePoint (Variables|/Game/SnappyRoads/Blueprints/BP_SnappyRoad.BP_SnappyRoad_C|GetSpline (Utilities|Array|Get(acopy) (Variables|Default|GetFollowPath) (Math|Integer|%(Integer) (+ (Variables|Default|GetCurrentRoad) 1) _returnvalue_2))) 0 "World") "World" true)
                      (Spline|SetTangentatSplinePoint _returnvalue_7 1 (* (Math|Vector|Normalize (Spline|GetTangentatSplinePoint (Variables|/Game/SnappyRoads/Blueprints/BP_SnappyRoad.BP_SnappyRoad_C|GetSpline (Utilities|Array|Get(acopy) (Variables|Default|GetFollowPath) (Math|Integer|%(Integer) (+ (Variables|Default|GetCurrentRoad) 1) _returnvalue_2))) 0 "World")) (Spline|GetSplineLength _returnvalue_7)) "World" true)
                      (Spline|SetTangentatSplinePoint _returnvalue_7 0 (* (Math|Vector|Normalize (Spline|GetTangentatSplinePoint (Variables|/Game/SnappyRoads/Blueprints/BP_SnappyRoad.BP_SnappyRoad_C|GetSpline (Utilities|Array|Get(acopy) _followpath (Variables|Default|GetCurrentRoad))) (- (Spline|GetNumberOfSplinePoints (Variables|/Game/SnappyRoads/Blueprints/BP_SnappyRoad.BP_SnappyRoad_C|GetSpline (Utilities|Array|Get(acopy) _followpath (Variables|Default|GetCurrentRoad)))) 1) "World")) (Spline|GetSplineLength _returnvalue_7)) "World" true)))))))
          (else
            (goto _label)))))
    (else
      (Actor|DestroyActor))))

(fn ConstructionScript)