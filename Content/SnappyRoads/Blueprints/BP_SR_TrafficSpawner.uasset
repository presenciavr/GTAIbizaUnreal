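; BP_SR_TrafficSpawner populates Snappy Roads paths with BP_SR_Vehicle traffic when play begins.
; A loop spawns vehicles at the origin, assigns the shared path and lane settings, cycles through the mesh list, and randomizes speed, lane, start road and time offset.
; Unless OneWay is set, it flips Reverse and reruns the same loop to add opposing traffic.
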(event EventBeginPlay
  (bind _vehiclemeshes (Variables|Default|GetVehicleMeshes))
  (Utilities|FlowControl|Sequence
    (:then_0
      (for _index (range 0 (Variables|Default|GetNumberOfCars)) :!label _label
        (bind _returnvalue (Game|SpawnActorfromClass "/Game/SnappyRoads/Blueprints/BP_SR_Vehicle.BP_SR_Vehicle_C" (Math|Transform|MakeTransform "0, 0, 0") "Undefined" 0 0))
        (Variables|/Game/SnappyRoads/Blueprints/BP_SR_Vehicle.BP_SR_Vehicle_C|SetFollowPath _returnvalue (Variables|Default|GetFollowPath))
        (Variables|/Game/SnappyRoads/Blueprints/BP_SR_Vehicle.BP_SR_Vehicle_C|SetSpeed%28km/h%29 _returnvalue (Math|Random|RandomFloatinRange (Variables|Default|GetMinSpeed) (Variables|Default|GetMaxSpeed)))
        (Variables|/Game/SnappyRoads/Blueprints/BP_SR_Vehicle.BP_SR_Vehicle_C|SetLane _returnvalue (Math|Random|RandomIntegerinRange (Variables|Default|GetMinLane) (Variables|Default|GetMaxLane)))
        (Variables|/Game/SnappyRoads/Blueprints/BP_SR_Vehicle.BP_SR_Vehicle_C|SetLineWidth _returnvalue (Variables|Default|GetLaneWidth))
        (Variables|/Game/SnappyRoads/Blueprints/BP_SR_Vehicle.BP_SR_Vehicle_C|SetOffset _returnvalue (Variables|Default|GetOffset))
        (Components|StaticMesh|SetStaticMesh (Variables|/Game/SnappyRoads/Blueprints/BP_SR_Vehicle.BP_SR_Vehicle_C|GetStaticMesh _returnvalue) (Utilities|Array|Get(acopy) _vehiclemeshes (Math|Integer|%(Integer) _index (Utilities|Array|Length _vehiclemeshes))))
        (Variables|/Game/SnappyRoads/Blueprints/BP_SR_Vehicle.BP_SR_Vehicle_C|SetReverse _returnvalue (Variables|Default|GetReverse))
        (Variables|/Game/SnappyRoads/Blueprints/BP_SR_Vehicle.BP_SR_Vehicle_C|SetTimeOffset _returnvalue (Math|Random|RandomFloatinRange 0.0 3e+01))
        (Variables|/Game/SnappyRoads/Blueprints/BP_SR_Vehicle.BP_SR_Vehicle_C|SetStartAtRoad _returnvalue (Math|Random|RandomIntegerinRange 0 (- (Utilities|Array|Length (Variables|Default|GetFollowPath)) 1)))))
    (:then_1
      (if (not (Variables|Default|GetOneWay))
        (Variables|Default|SetReverse (not (Variables|Default|GetReverse)))
        (goto _label)))))

(event Collision|EventActorBeginOverlap
  (params (OtherActor :type Actor%20Object%20Reference)))

(event EventTick
  (params (DeltaSeconds :type Float%20%28single-precision%29)))

(fn ConstructionScript)