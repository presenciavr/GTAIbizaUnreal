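; BP_pausa is a Blueprint that toggles the game's pause menu through its PausarPartida function.
; The function finds the Ui_menupause and Ui_principal widgets and swaps their visibility based on the Menupause flag.
; It also switches input mode and cursor display, and clears hover on the Continuar and Salir texts when leaving.
; It does not call SetGamePaused, so only UI and input change here.
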(fn ConstructionScript)

(fn PausarPartida
  (bind _returnvalue (Game|GetPlayerController 0))
  ;[1 1 1] Funcion que activa la Pausa. Oculta la uiprincipal y hace visible el pause
  (Utilities|FlowControl|Sequence
    (:then_0
      (bind _foundwidgets (Widget|GetAllWidgetsOfClass "/Game/Personas/Gabri/Menupause/ui_menupause.ui_menupause_C" true)))
    (:then_1
      (bind _foundwidgets_2 (Widget|GetAllWidgetsOfClass "/Game/Personas/Gabri/UIPrincipal/ui_principal.ui_principal_C" true)))
    (:then_2
      (if (Variables|Default|Getmenupause) ; Comprobamos si estamos o no en el menu pausa
        (Variables|Default|Setmenupause false) ; Salimos del Menu Pausa
        (Default|Unhover (Utilities|Array|Get(acopy) _foundwidgets) (Variables|/Game/Personas/Gabri/Menupause/ui_menupause.ui_menupause_C|Gettext_continuar (Utilities|Array|Get(acopy) _foundwidgets)))
        (Default|Unhover (Utilities|Array|Get(acopy) _foundwidgets) (Variables|/Game/Personas/Gabri/Menupause/ui_menupause.ui_menupause_C|Gettext_salir (Utilities|Array|Get(acopy) _foundwidgets)))
        (Widget|SetVisibility (Utilities|Array|Get(acopy) _foundwidgets_2) "Visible")
        (Widget|SetVisibility (Utilities|Array|Get(acopy) _foundwidgets) "Hidden")
        (Input|SetInputModeGameOnly _returnvalue)
        (else
          (Variables|Default|Setmenupause true) ; Entramos al Menu Pausa
          (Widget|SetVisibility (Utilities|Array|Get(acopy) _foundwidgets_2) "Hidden")
          (Widget|SetVisibility (Utilities|Array|Get(acopy) _foundwidgets) "Visible")
          (Input|SetInputModeGameandUI _returnvalue 0 "DoNotLock" false)))
      (Variables|/Script/Engine.PlayerController|SetbShowMouseCursor _returnvalue (Variables|Default|Getmenupause)))))