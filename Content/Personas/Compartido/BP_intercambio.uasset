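; Shared character Blueprint that tracks the equipped weapon and health, with functions to switch between three weapons and receive damage.
; Each equip function branches on the current weapon, updates it and plays the matching swap animation on the Ui_principal widget, found by class lookup.
; One animation per weapon pair covers both directions through forward or reverse playback.
; Damage is simply subtracted from health, without clamping, and the event graph is empty.
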(event EventBeginPlay)

(event Collision|EventActorBeginOverlap
  (params (OtherActor :type Actor%20Object%20Reference)))

(event EventTick
  (params (DeltaSeconds :type Float%20%28single-precision%29)))

(fn ConstructionScript)

(fn EquiparArma1
  ;[1 1 1] Funcion que cambia al Arma1 y ejecuta la animacion dependiendo del arma que tuvieramos equipada
  (switch int (Variables|Default|Getarmaequipada)
    (:2
      (Variables|Default|Setarmaequipada 1) ; Configuramos el arma elegida
      (bind _foundwidgets (Widget|GetAllWidgetsOfClass "/Game/Personas/Gabri/UIPrincipal/ui_principal.ui_principal_C" true)) ; Ejecutamos la animacion de cambio de arma correspondiente, dependiendo del arma que teniamos y la que estamos equipando
      (UserInterface|Animation|PlayAnimation (Utilities|Array|Get(acopy) _foundwidgets) (Variables|/Game/Personas/Gabri/UIPrincipal/ui_principal.ui_principal_C|GetAnim_ui_cambioarma12 (Utilities|Array|Get(acopy) _foundwidgets)) 0.0 1 "Reverse" 1.0))
    (:3
      (Variables|Default|Setarmaequipada 1)
      (bind _foundwidgets_2 (Widget|GetAllWidgetsOfClass "/Game/Personas/Gabri/UIPrincipal/ui_principal.ui_principal_C" true))
      (UserInterface|Animation|PlayAnimation (Utilities|Array|Get(acopy) _foundwidgets_2) (Variables|/Game/Personas/Gabri/UIPrincipal/ui_principal.ui_principal_C|GetAnim_ui_cambioarma13 (Utilities|Array|Get(acopy) _foundwidgets_2)) 0.0 1 "Reverse" 1.0))))

(fn EquiparArma2
  ;[1 1 1] Funcion que cambia al Arma2 y ejecuta la animacion dependiendo del arma que tuvieramos equipada
  (switch int (Variables|Default|Getarmaequipada)
    (:1
      (Variables|Default|Setarmaequipada 2)
      (bind _foundwidgets (Widget|GetAllWidgetsOfClass "/Game/Personas/Gabri/UIPrincipal/ui_principal.ui_principal_C" true))
      (UserInterface|Animation|PlayAnimation (Utilities|Array|Get(acopy) _foundwidgets) (Variables|/Game/Personas/Gabri/UIPrincipal/ui_principal.ui_principal_C|GetAnim_ui_cambioarma12 (Utilities|Array|Get(acopy) _foundwidgets)) 0.0 1 "Forward" 1.0))
    (:3
      (Variables|Default|Setarmaequipada 2)
      (bind _foundwidgets_2 (Widget|GetAllWidgetsOfClass "/Game/Personas/Gabri/UIPrincipal/ui_principal.ui_principal_C" true))
      (UserInterface|Animation|PlayAnimation (Utilities|Array|Get(acopy) _foundwidgets_2) (Variables|/Game/Personas/Gabri/UIPrincipal/ui_principal.ui_principal_C|GetAnim_ui_cambioarma23 (Utilities|Array|Get(acopy) _foundwidgets_2)) 0.0 1 "Reverse" 1.0))))

(fn EquiparArma3
  ;[1 1 1] Funcion que cambia al Arma3 y ejecuta la animacion dependiendo del arma que tuvieramos equipada
  (switch int (Variables|Default|Getarmaequipada)
    (:1
      (Variables|Default|Setarmaequipada 3)
      (bind _foundwidgets (Widget|GetAllWidgetsOfClass "/Game/Personas/Gabri/UIPrincipal/ui_principal.ui_principal_C" true))
      (UserInterface|Animation|PlayAnimation (Utilities|Array|Get(acopy) _foundwidgets) (Variables|/Game/Personas/Gabri/UIPrincipal/ui_principal.ui_principal_C|GetAnim_ui_cambioarma13 (Utilities|Array|Get(acopy) _foundwidgets)) 0.0 1 "Forward" 1.0))
    (:2
      (Variables|Default|Setarmaequipada 3)
      (bind _foundwidgets_2 (Widget|GetAllWidgetsOfClass "/Game/Personas/Gabri/UIPrincipal/ui_principal.ui_principal_C" true))
      (UserInterface|Animation|PlayAnimation (Utilities|Array|Get(acopy) _foundwidgets_2) (Variables|/Game/Personas/Gabri/UIPrincipal/ui_principal.ui_principal_C|GetAnim_ui_cambioarma23 (Utilities|Array|Get(acopy) _foundwidgets_2)) 0.0 1 "Forward" 1.0))))

(fn RecibirDanyo
  (params (danyo :type Integer))
  ;[1 1 1] Funcion que modifica el valor de la salud en funcion del danyo
  (Variables|Default|Setsalud (- (Variables|Default|Getsalud) danyo)) ; Actualizamos Valor Real de la salud  del personaje segun el danyo
)