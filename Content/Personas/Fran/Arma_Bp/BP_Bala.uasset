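; BP_Bala is a physics-driven bullet that reports hits on ThirdPersonCharacterManu characters.
; BeginPlay scales speed by RatioVelocidad and divides mass by its square, preserving kinetic energy, then overrides the Sphere's mass in kilograms.
; Disparar launches the Sphere along the root's forward vector with a mass-times-velocity impulse in Unreal units.
; On hit, it passes the hit result, current velocity and mass to the character's RecibeGolpe.
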(event EventBeginPlay
  (bind _ratiovelocidad (Variables|Default|GetRatioVelocidad))
  (Variables|Default|SetVelocidad (* (Variables|Default|GetVelocidad) _ratiovelocidad))
  (bind _output_get (Variables|Default|SetMasa (/ (Variables|Default|GetMasa) (* _ratiovelocidad (Variables|Default|GetRatioVelocidad)))))
  (Class|PrimitiveComponent|SetMassOverrideinKg (Variables|Default|GetSphere) "None" (/ _output_get 1e+03) true))

(event Collision|EventHit
  (params (MyComp :type Primitive%20Component%20Object%20Reference) (Other :type Actor%20Object%20Reference) (OtherComp :type Primitive%20Component%20Object%20Reference) (bSelfMoved :type Boolean) (HitLocation :type Vector :default "0, 0, 0") (HitNormal :type Vector :default "0, 0, 0") (NormalImpulse :type Vector :default "0, 0, 0") (Hit :type Hit%20Result%20Structure%20%28by%20ref%29))
  (bind _sphere (Variables|Default|GetSphere))
  ;[1 1 1] Al colisionar con un personaje se llama al evento recibir golpe
  (bind _asthird_person_character_manu (Utilities|Casting|CastToThirdPersonCharacterManu Other))
  (Default|RecibeGolpe _asthird_person_character_manu Hit (Transformation|GetComponentVelocity _sphere) (Physics|GetMass _sphere)))

(fn ConstructionScript)

(fn Disparar
  (bind _sphere (Variables|Default|GetSphere))
  (Physics|AddImpulse _sphere (* (Math|Vector|GetForwardVector (Variables|Default|GetDefaultSceneRoot)) (* (Physics|GetMass _sphere) (* (Variables|Default|GetVelocidad) 1e+02))) "None" false))