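; Multiplayer socket client actor that connects to a hard-coded LAN TCP server on BeginPlay and closes the connection on EndPlay.
; A Delay on Tick throttles sending to roughly five messages per second.
; Each message is one letter-tagged string holding the player capsule's location and rotation, plus health and equipped weapon from the first BP_intercambio actor.
; Connection status is only printed; incoming data is not handled here.
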(event Custom|CustomEvent_0
  (params (success :type Boolean) (message :type String))
  ;[1 1 1] Arranca conexion con el servidor
  (if success
    (Development|PrintString "CONEXION ESTABLECIDA" true true "(R=0.125954,G=1.000000,B=0.000000,A=1.000000)" 5.0)
    (else
      (Development|PrintString "SE HA PERDIDO LA CONEXION" true true "(R=0.885417,G=0.000000,B=0.008455,A=1.000000)" 2e+01))))

(event EventBeginPlay
  (bind _returnvalue (Class|SocketClientHandler|GetSocketClientTarget))
  ;[1 1 1] Arranca conexion con el servidor
  (Class|SocketClientBPLibrary|ConnectSocketClient _returnvalue "192.168.1.67" 12345)
  (EventDispatchers|BindEventtoOnsocketClientConnectionEventDelegate _returnvalue (delegate Custom|CustomEvent_0)))

(event EventEndPlay
  (params (EndPlayReason :type EEndPlayReason%20Enum :default "Destroyed"))
  ;[1 1 1] Cerramos la conexion al cerrar el juego
  (Class|SocketClientBPLibrary|CloseSocketClientConnection (Class|SocketClientHandler|GetSocketClientTarget)))

(event EventTick
  (params (DeltaSeconds :type Float%20%28single-precision%29))
  ;[1 1 1] Enviar Informacion al Servidor
  (Utilities|FlowControl|Delay 0.2)
  (Utilities|FlowControl|Sequence
    (:then_0
      (bind _asthird_person_character_manu (Utilities|Casting|CastToThirdPersonCharacterManu (Game|GetPlayerCharacter 0))))
    (:then_1
      (bind _outactors (Actor|GetAllActorsOfClass "/Game/Personas/Compartido/BP_intercambio.BP_intercambio_C"))
      (Class|SocketClientBPLibrary|SocketClientSendTCPMessage (Utilities|String|Append "X" (Utilities|String|ToString(Float) (.x (Transformation|GetWorldLocation (Variables|/Script/Engine.Character|GetCapsuleComponent _asthird_person_character_manu)))) "Y" (Utilities|String|ToString(Float) (.y (Transformation|GetWorldLocation (Variables|/Script/Engine.Character|GetCapsuleComponent _asthird_person_character_manu)))) "Z" (Utilities|String|ToString(Float) (.z (Transformation|GetWorldLocation (Variables|/Script/Engine.Character|GetCapsuleComponent _asthird_person_character_manu)))) "R" (Utilities|String|ToString(Float) (.roll (Transformation|GetWorldRotation (Variables|/Script/Engine.Character|GetCapsuleComponent _asthird_person_character_manu)))) "P" (Utilities|String|ToString(Float) (.pitch (Transformation|GetWorldRotation (Variables|/Script/Engine.Character|GetCapsuleComponent _asthird_person_character_manu)))) "W" (Utilities|String|ToString(Float) (.yaw (Transformation|GetWorldRotation (Variables|/Script/Engine.Character|GetCapsuleComponent _asthird_person_character_manu)))) "S" (Utilities|String|ToString(Integer) (Variables|/Game/Personas/Compartido/BP_intercambio.BP_intercambio_C|Getsalud (Utilities|Array|Get(acopy) _outactors))) "A" (Utilities|String|ToString(Integer) (Variables|/Game/Personas/Compartido/BP_intercambio.BP_intercambio_C|Getarmaequipada (Utilities|Array|Get(acopy) _outactors)))) 0 true))))

(fn ConstructionScript)