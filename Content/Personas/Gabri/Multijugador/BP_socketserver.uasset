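; BP_socketserver is a test TCP server for multiplayer that uses a socket server plugin target.
; Key 5 starts the server on a hardcoded LAN IP and port, then binds its connection and message-received delegates.
; Connection events print the status message for the server or the session ID for clients, and received messages print with their sender's session ID.
; Key 6 stops the server.
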(event Custom|CustomEvent_0
  (params (type :type EServerSocketConnectionEventType%20Enum :default "E_Server") (success :type Boolean) (message :type String) (sessionID :type String))
  ;[1 1 1] Inicia el servidor y escucha
  (switch Utilities|FlowControl|Switch|SwitchonEServerSocketConnectionEventType type
    (:E_Server
      (Development|PrintString message true true "(R=0.000000,G=0.660000,B=1.000000,A=1.000000)" 5.0))
    (:E_Client
      (Development|PrintString sessionID true true "(R=0.000000,G=0.660000,B=1.000000,A=1.000000)" 5.0))))

(event Custom|CustomEvent_1
  (params (sessionID :type String) (message :type String) (byteArray :type Array%20of%20Bytes))
  ;[1 1 1] Inicia el servidor y escucha
  (Development|PrintString (Utilities|String|Append "El ordenador " sessionID " ha dicho: " message)))

(event Input|KeyboardEvents|5
  (params (Key :type Key%20Structure))
  (bind _returnvalue (Class|SocketServerBPLibrary|GetSocketServerTarget))
  ;[1 1 1] Inicia el servidor y escucha
  (:Pressed
    (Class|SocketServerBPLibrary|StartTCPServer _returnvalue "192.168.1.106" 12345)
    (EventDispatchers|BindEventtoOnsocketServerConnectionEventDelegate _returnvalue (delegate Custom|CustomEvent_0))
    (EventDispatchers|BindEventtoOnserverReceiveTCPMessageEventDelegate _returnvalue (delegate Custom|CustomEvent_1))))

(event Input|KeyboardEvents|6
  (params (Key :type Key%20Structure))
  ;[1 1 1] Apaga el servidor
  (:Pressed
    (Class|SocketServerBPLibrary|StopTCPServer (Class|SocketServerBPLibrary|GetSocketServerTarget))))

(fn ConstructionScript)